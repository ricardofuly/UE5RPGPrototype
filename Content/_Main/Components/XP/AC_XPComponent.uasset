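; Actor component that tracks XP and level for its owner and rewards XP to whoever kills it.
; AwardXP adds to a cumulative total, then recursively levels up against CT_Levels curve thresholds until short or at MaxLevel.
; Each level-up broadcasts OnLeveledUp, which refreshes the owner's XP bounty from the same curve table.
; On a State.Dead gameplay tag change, that bounty goes to the originating controller's pawn's XP component.
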(event Custom|RewardOnDie
  (params (GameplayTagContext :type F%20Gameplay%20Context%20Structure))
  (bind (_activetags _origin) (Utilities|Struct|BreakF_GameplayContext GameplayTagContext))
  (bind _controller (Utilities|Struct|BreakF_Origin _origin))
  (bind _returnvalue (Pawn|GetControlledPawn _controller))
  (bind _returnvalue_2 (Actor|GetComponentbyClass _returnvalue "AC_XPComponent_C"))
  (if (GameplayTags|HasTag _activetags "(TagName=\"State.Dead\")")
    (Utilities|IsValid _controller
      (:Is%20Valid
        (Utilities|IsValid _returnvalue_2
          (:Is%20Valid
            (CallFunction|AwardXP _returnvalue_2 (Variables|Default|GetXPToAward))))))))

(event Custom|AwardXP
  (params (AwardedXP :type Float%20%28double-precision%29))
  (Variables|Default|SetCurrentXP (+ (Variables|Default|GetCurrentXP) AwardedXP))
  (CallFunction|TrytoLevelUp))

(event Custom|OnLevelUp
  (params (NewLevel :type Integer))
  (CallFunction|SetCurrentXPAwarded))

(event EventBeginPlay
  (CallFunction|SetCurrentXPAwarded)
  (CallFunction|TrytoLevelUp)
  (EventDispatchers|BindEventtoOnStateChange (Actor|GetComponentbyClass (Components|GetOwner) "/Game/_Main/Components/GameplayTags/AC_GameplayTags.AC_GameplayTags_C") (EventDispatchers|CreateEvent :!event Custom|RewardOnDie))
  (EventDispatchers|BindEventtoOnLeveledUp (EventDispatchers|CreateEvent :!event Custom|OnLevelUp))
  (Default|CallOnLeveledUp (Variables|Default|GetCurrentLevel)))

(event EventTick
  (params (DeltaSeconds :type Float%20%28single-precision%29)))

(fn TrytoLevelUp
  (bind _leveledup (CallFunction|LevelUp?))
  (if _leveledup
    (Development|PrintString "Leveled Up!")
    (CallFunction|TrytoLevelUp)
    (return)
    (else
      (return))))

(fn LevelUp?
  (if (== (Variables|Default|GetCurrentLevel) (Variables|Default|GetMaxLevel))
    (return false)
    (else
      (bind _outxy (DataTable|EvaluateCurveTableRow "/Game/_Main/Components/XP/CT_Levels.CT_Levels" "LevelXP" (Math|Conversions|ToFloat(Integer) (+ (Variables|Default|GetCurrentLevel) 1)))
        (:RowFound
          (Variables|Default|SetNextLevelXP _outxy)
          (if (>= (Variables|Default|GetCurrentXP) _outxy)
            (bind _output_get (Variables|Default|SetCurrentLevel (+ (Variables|Default|GetCurrentLevel) 1)))
            (Default|CallOnLeveledUp _output_get)
            (return true)
            (else
              (return false))))
        (:RowNotFound
          (return false))))))

(fn SetCurrentXPAwarded
  (bind _outxy (DataTable|EvaluateCurveTableRow "/Game/_Main/Components/XP/CT_Levels.CT_Levels" "AwardedXP" (Math|Conversions|ToFloat(Integer) (+ (Variables|Default|GetCurrentLevel) 1)))
    (:RowFound
      (Variables|Default|SetXPToAward _outxy)
      (return))
    (:RowNotFound
      (return))))

(fn GetXPValues)

(fn GetCurrentLevel
  (return (Variables|Default|GetCurrentLevel)))