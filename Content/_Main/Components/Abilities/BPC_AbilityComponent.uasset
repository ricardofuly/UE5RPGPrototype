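; BPC_AbilityComponent is a pawn component that grants abilities and triggers their use.
; It caches the owning Pawn on BeginPlay, then spawns each ability class as an actor with that pawn as Owner and Instigator.
; Spawned abilities are stored in AvaliableAbilities, and each addition broadcasts OnAvaliableAbilitiesChanged.
; InitializeAbilities adds a list of known classes, and UseAbility calls AttemptUseAbility on the ability at a given index.
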(event EventBeginPlay
  (bind _aspawn (Utilities|Casting|CastToPawn (Components|GetOwner)))
  (Variables|Default|SetOwnerPawn _aspawn))

(fn AddAbilitybyClass
  (params (AbilityClass :type BP%20Ability%20Class%20Reference))
  (bind _ownerpawn (Variables|Default|GetOwnerPawn))
  (bind _returnvalue (Game|SpawnActorfromClass AbilityClass (Math|Transform|MakeTransform "0, 0, 0" "0, 0, 0" "1.000000,1.000000,1.000000") "Undefined" "MultiplyWithRoot" _ownerpawn _ownerpawn))
  (Utilities|Array|Add (Variables|Default|GetAvaliableAbilities) _returnvalue)
  (Default|CallOnAvaliableAbilitiesChanged (Variables|Default|GetAvaliableAbilities))
  (return))

(fn UseAbility
  (params (AbilityIndex :type Integer))
  (Default|AttemptUseAbility (Utilities|Array|Get(acopy) (Variables|Default|GetAvaliableAbilities) AbilityIndex))
  (return))

(fn InitializeAbilities
  (params (KnownAbilities :type Array%20of%20BP%20Ability%20Class%20References))
  (for _array_element KnownAbilities
    (CallFunction|AddAbilitybyClass _array_element))
  (return))