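; BP_Ability is an ability component that plays a montage on its owner's character mesh when used.
; An attempt runs an event chain from AttemptUseAbility through UseAbilityPreStep to UseAbility, behind a condition that is always true here.
; EndAbility runs when the montage completes or is interrupted, or immediately if the mesh or montage is invalid.
; EndAbility and construction are empty, and the file sets no cooldown or cost.
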(event Custom|AttemptUseAbility
  (if true
    (CallFunction|UseAbilityPreStep)))

(event Custom|UseAbility
  (bind _returnvalue (Components|GetOwner))
  (bind _returnvalue_2 (CallFunction|GetCharacterMesh _returnvalue))
  (Utilities|IsValid _returnvalue_2
    (:Is%20Valid
      (bind _abilitymontage (Variables|Default|GetAbilityMontage)
        (:then
          (Animation|Montage|PlayMontage _returnvalue_2 _abilitymontage
            (:OnCompleted
              _)
            (:OnInterrupted
              _))
          (CallFunction|EndAbility))
        (:else
          (CallFunction|EndAbility :!label _label))))
    (:Is%20Not%20Valid
      (goto _label))))

(event Custom|UseAbilityPreStep
  (CallFunction|UseAbility))

(event Custom|EndAbility)

(event EventBeginPlay)

(fn ConstructionScript)