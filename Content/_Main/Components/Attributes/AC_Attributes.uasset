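; Actor component that holds gameplay attributes as structs looked up by gameplay tag, with Health the only one handled.
; ChangeAttribute routes by tag to ChangeAttributeValue, which adds the change to the chosen Base Value, Delta, Multiplier or Max field without clamping.
; The resulting context, carrying attribute, change and origin, is broadcast through OnAttributeChange.
; BeginPlay also broadcasts Health to publish its initial state.
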(event EventBeginPlay
  (Default|CallOnAttributeChange "(TagName=\"Attribute.Health\")" (Utilities|Struct|MakeF_AttributeContext (Variables|Default|GetHealth))))

(fn GetAttributefromTag
  (params (TagSearchFor :type Gameplay%20Tag%20Structure))
  (|SwitchGameplayTag TagSearchFor
    (:Attribute.Health
      (bind _output_get (LocalVariables|SetLocalAttribute (Variables|Default|GetHealth)))
      (return _output_get))))

(fn ChangeAttribute
  (params (AttributeTag :type Gameplay%20Tag%20Structure) (ValueChange :type Float%20%28double-precision%29) (AttributeTypeToChange :type E_Attribute%20Enum :default "NewEnumerator0") (Origin :type F%20Origin%20Structure))
  (|SwitchGameplayTag AttributeTag
    (:Attribute.Health
      (bind _attributecontext (CallFunction|ChangeAttributeValue (Variables|Default|GetHealth) ValueChange AttributeTypeToChange Origin))
      (Default|CallOnAttributeChange AttributeTag _attributecontext))))

(fn ChangeAttributeValue
  (params (AttributeToChange :type F%20Attributes%20Structure%20%28by%20ref%29) (ValueChange :type Float%20%28double-precision%29) (AttributeTypeToChange :type E_Attribute%20Enum :default "NewEnumerator0") (Origin :type F%20Origin%20Structure))
  (bind (_basevalue _delta _multiplier _max) (Utilities|Struct|BreakF_Attributes AttributeToChange))
  (switch Utilities|FlowControl|Switch|SwitchonE_Attribute AttributeTypeToChange
    (:NewEnumerator0
      (return ""))
    (:NewEnumerator1
      (Utilities|Struct|SetmembersinF_Attributes AttributeToChange (+ _basevalue ValueChange))
      (return (Utilities|Struct|MakeF_AttributeContext AttributeToChange ValueChange Origin)))
    (:NewEnumerator2
      (Utilities|Struct|SetmembersinF_Attributes AttributeToChange (+ ValueChange _delta))
      (return (Utilities|Struct|MakeF_AttributeContext AttributeToChange ValueChange Origin)))
    (:NewEnumerator3
      (Utilities|Struct|SetmembersinF_Attributes AttributeToChange (+ ValueChange _multiplier))
      (return (Utilities|Struct|MakeF_AttributeContext AttributeToChange ValueChange Origin)))
    (:NewEnumerator4
      (Utilities|Struct|SetmembersinF_Attributes AttributeToChange (+ ValueChange _max))
      (return (Utilities|Struct|MakeF_AttributeContext AttributeToChange ValueChange Origin)))))