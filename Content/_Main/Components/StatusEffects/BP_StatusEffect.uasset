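; Base status effect that applies timed gameplay tags and attribute changes through components on the owner's instigator controller.
; AttemptToApply checks required and preventing tags, then either starts the effect with periodic and duration timers or removes it from the StatusEffectComponent.
; Attribute changes scale by curve tables at player or effect level and are applied negated on end, alongside tag removal and timer cleanup.
; PeriodicEvent is empty here.
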(event Custom|AttemptToApply
  (if (CallFunction|CheckTagStartConditions)
    (CallFunction|StartStatusEffect)
    (else
      (CallFunction|AttempRemoveStatusEffect))))

(event Custom|StartStatusEffect
  (bind _statuseffectinfo (Variables|Default|GetStatusEffectInfo))
  (bind _statuseffectsinfo (Variables|/Game/_Main/Components/StatusEffects/Data/PrimaryData/PDA_StatusEffectsData.PDA_StatusEffectsData_C|GetStatusEffectsInfo _statuseffectinfo))
  (bind (_duration _periodictime) (Utilities|Struct|BreakF_StatusEffects _statuseffectsinfo))
  (CallFunction|AddTags)
  (CallFunction|ApplyAttributeEffects true)
  (bind _returnvalue (Utilities|Time|SetTimerbyEvent (EventDispatchers|CreateEvent :!event Custom|PeriodicEvent) _periodictime true))
  (Variables|Default|SetPeriodicTimerHandle _returnvalue)
  (bind _returnvalue_2 (Utilities|Time|SetTimerbyEvent (EventDispatchers|CreateEvent :!event Custom|EndStatusEffect) _duration false false 0.001))
  (Variables|Default|SetDurationTimerHandle _returnvalue_2))

(event Custom|PeriodicEvent)

(event Custom|EndStatusEffect
  (CallFunction|RemoveTags)
  (CallFunction|ApplyAttributeEffects false)
  (CallFunction|ClearTimers)
  (CallFunction|AttempRemoveStatusEffect))

(event EventBeginPlay)

(fn ConstructionScript)

(fn ClearTimers
  (Utilities|Time|ClearandInvalidateTimerbyHandle (Variables|Default|GetPeriodicTimerHandle))
  (Utilities|Time|ClearandInvalidateTimerbyHandle (Variables|Default|GetDurationTimerHandle))
  (return))

(fn CheckTagStartConditions
  (bind _returnvalue (Components|GetOwner))
  (bind _returnvalue_2 (Game|GetInstigatorController _returnvalue))
  (bind _returnvalue_3 (CallFunction|GetGameplayTagComponent _returnvalue_2))
  (bind _returnvalue_4 (Default|GetActiveTagContainer _returnvalue_3))
  (return (and (GameplayTags|HasAllTags _returnvalue_4 (Variables|Default|GetRequiredTags)) (not (GameplayTags|HasAnyTags _returnvalue_4 (Variables|Default|GetPreventingTags))))))

(fn AttempRemoveStatusEffect
  (Default|RemoveStatusEffect (CallFunction|GetStatusEffectComponent (Game|GetInstigatorController (Components|GetOwner))) self)
  (return))

(fn AddTags
  (bind _returnvalue (Components|GetOwner))
  (for _array_element (Variables|Default|GetAddingTags)
    (Default|AddTag (CallFunction|GetGameplayTagComponent (Game|GetInstigatorController _returnvalue)) _array_element (CallFunction|MakeOrigin _returnvalue)))
  (return))

(fn RemoveTags
  (bind _returnvalue (Components|GetOwner))
  (for _array_element (Variables|Default|GetAddingTags)
    (Default|RemoveTag (CallFunction|GetGameplayTagComponent (Game|GetInstigatorController _returnvalue)) _array_element (CallFunction|MakeOrigin _returnvalue)))
  (return))

(fn ApplyAttributeEffects
  (params (AddEffect :type Boolean))
  (bind _returnvalue (Components|GetOwner))
  (bind _returnvalue_2 (Game|GetInstigatorController _returnvalue))
  (if AddEffect
    (LocalVariables|SetL_AttributeMultiplier 1.0)
    (else
      (LocalVariables|SetL_AttributeMultiplier -1.0)))
  (for _array_element (Variables|Default|GetAttributeEffects)
    (bind _outxy (DataTable|EvaluateCurveTableRow (.CurveTable (Utilities|Struct|BreakCurveTableRowHandle (.ScalingCurve (Utilities|Struct|BreakF_AttributeChange _array_element)))) (.RowName (Utilities|Struct|BreakCurveTableRowHandle (.ScalingCurve (Utilities|Struct|BreakF_AttributeChange _array_element)))) (select (Variables|Default|GetUsePlayerLevel) (Math|Conversions|ToFloat(Integer) (Default|GetCurrentLevel (CallFunction|GetXPComponent _returnvalue_2))) (Variables|Default|GetEffectLevel)))
      (:RowFound
        (Default|ChangeAttribute (CallFunction|GetAttributeComponent _returnvalue_2) (.AttributeToChange (Utilities|Struct|BreakF_AttributeChange _array_element)) (* (* (.PowerMultiplier (Utilities|Struct|BreakF_AttributeChange _array_element)) _outxy) (LocalVariables|GetL_AttributeMultiplier)) (.AttributeType (Utilities|Struct|BreakF_AttributeChange _array_element)) (CallFunction|MakeOrigin _returnvalue)))))
  (return))