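; BP_Player is the player character Blueprint, wiring gameplay tag, attribute and status effect components to debug key tests.
; On BeginPlay it binds to tag state changes and prints a death message when State.Dead is active.
; Number keys add the dead tag, reduce health, or spawn and apply a BP_HealthPointLoss status effect.
; The attribute-change handler switches on the tag but has no actions attached.
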(event OnAttributeChange(AttributesComponent)
  (params (AttributeTag :type Gameplay%20Tag%20Structure) (AttributeContext :type F%20Attribute%20Context%20Structure))
  (|SwitchGameplayTag AttributeTag))

(event Custom|OnDead
  (params (GameplayTagContext :type F%20Gameplay%20Context%20Structure))
  (if (GameplayTags|HasTag (.ActiveTags (Utilities|Struct|BreakF_GameplayContext GameplayTagContext)) "(TagName=\"State.Dead\")")
    (Development|PrintString "You're dead ma boy!")))

(event EventBeginPlay
  (EventDispatchers|BindEventtoOnStateChange (Variables|Default|GetGameplayTag%20Component) (delegate Custom|OnDead)))

(event Input|KeyboardEvents|3
  (params (Key :type Key%20Structure :default "None"))
  (bind _self self)
  (:Pressed
    (bind _returnvalue (Game|SpawnActorfromClass "/Game/_Main/Components/StatusEffects/Health/BP_HealthPointLoss.BP_HealthPointLoss_C" (Math|Transform|MakeTransform "0, 0, 0" "0, 0, 0" "1.000000,1.000000,1.000000") "Undefined" "MultiplyWithRoot" _self _self))
    (Default|AddStatusEffect (Variables|Default|GetStatus%20Effect%20Component) _returnvalue)))

(event Input|KeyboardEvents|1
  (params (Key :type Key%20Structure :default "None"))
  (:Pressed
    (Default|AddTag (Variables|Default|GetGameplayTag%20Component) "(TagName=\"State.Dead\")" (CallFunction|MakeOrigin self))))

(event Input|KeyboardEvents|2
  (params (Key :type Key%20Structure :default "None"))
  (:Pressed
    (Default|ChangeAttribute (Variables|Default|GetAttributes%20Component) "(TagName=\"Attribute.Health\")" -2e+01 "NewEnumerator1" (CallFunction|MakeOrigin self))))

(fn ConstructionScript
  (|CallParentFunction))