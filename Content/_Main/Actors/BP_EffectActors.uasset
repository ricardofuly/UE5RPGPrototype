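; BP_EffectActors is a trigger actor that grants a configurable status effect to whoever overlaps its box.
; On overlap it spawns EffectClass, owned by the overlapping actor, and passes it to the instigator controller's status effect component.
; The construction script sets the label text, and BeginPlay creates a dynamic icon material on Fill.
; A fill-progress timeline ending in a particle burst is present but never runs.
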(event OnComponentBeginOverlap(TriggerBox)
  (params (OverlappedComponent :type Primitive%20Component%20Object%20Reference) (OtherActor :type Actor%20Object%20Reference) (OtherComp :type Primitive%20Component%20Object%20Reference) (OtherBodyIndex :type Integer) (bFromSweep :type Boolean) (SweepResult :type Hit%20Result%20Structure%20%28by%20ref%29))
  (bind _returnvalue (Game|SpawnActorfromClass (Variables|Default|GetEffectClass) (Math|Transform|MakeTransform "0, 0, 0" "0, 0, 0" "1.000000,1.000000,1.000000") "Undefined" "MultiplyWithRoot" OtherActor (Variables|/Script/Engine.Actor|GetInstigator OtherActor)))
  (Default|AddStatusEffect (CallFunction|GetStatusEffectComponent (Game|GetInstigatorController OtherActor)) _returnvalue))

(event EventBeginPlay
  (Rendering|Material|SetMaterial (Variables|Default|GetFill) 0 (Variables|Default|GetIconMaterial))
  (bind _returnvalue (Rendering|Material|CreateDynamicMaterialInstance (Variables|Default|GetFill) 0 (Variables|Default|GetIconMaterial) "None" :!class /Script/Engine.PrimitiveComponent))
  (Variables|Default|SetEffectMaterialInstance _returnvalue))

(event Collision|EventActorBeginOverlap
  (params (OtherActor :type Actor%20Object%20Reference)))

(event EventTick
  (params (DeltaSeconds :type Float%20%28single-precision%29)))

(fn ConstructionScript
  (Rendering|Components|TextRender|SetText (Variables|Default|GetTextRender) (Variables|Default|GetEffectText)))